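; Spiked roller hazard for a platformer that knocks the first-person player away on overlap.
; UpnDown and LeftAndRight flags each add an InterpToMovement component at BeginPlay, while Rotate spins the actor around its local roll axis every Tick.
; Overlap launches the player opposite their own facing and upward, with a camera shake and damage sound at their location.
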(event EventBeginPlay
  (if (Variables|Default|Get¿UpnDown?)
    (AddComponent|AddInterptoMovementComponent))
  (if (Variables|Default|GetLeftAndRight?)
    (AddComponent|AddInterptoMovementComponent)))

(event Collision|EventActorBeginOverlap
  (params (OtherActor :type Actor%20Object%20Reference))
  (bind _returnvalue (Game|GetPlayerCharacter 0))
  (bind _returnvalue_2 (Game|GetPlayerCharacter 0))
  (bind _returnvalue_3 (Transformation|GetActorLocation _returnvalue))
  (Utilities|Casting|CastToFirstPersonCharacter OtherActor)
  (Character|LaunchCharacter _returnvalue_2 (+ (* (Math|Vector|NegateVector (Math|Vector|GetForwardVector (Variables|/Script/Engine.Actor|GetRootComponent _returnvalue_2))) 3000) "0,0.000000,1500.000000") false false)
  (Camera|PlayWorldCameraShake "/Script/Engine.MatineeCameraShake" _returnvalue_3 1.0 5e+02)
  (Audio|PlaySoundatLocation "/Game/SFX/Minecraft_Damage__Oof__-_Sound_Effect__HD_.Minecraft_Damage__Oof__-_Sound_Effect__HD_" _returnvalue_3 "0, 0, 0" 1.0 1.0 0.0 0 0 0) ; Play firing sound
)

(event EventTick
  (params (DeltaSeconds :type Float%20%28single-precision%29))
  (if (Variables|Default|GetRotate?)
    (Transformation|AddActorLocalRotation (Math|Rotator|MakeRotator (* 200 DeltaSeconds) 0.0 0.0) false false)))

(fn ConstructionScript)