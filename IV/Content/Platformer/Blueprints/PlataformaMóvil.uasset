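; Moving platform actor for a platformer, with flags that select vertical, sideways or rotating motion.
; On BeginPlay, the UpnDown and LeftAndRight flags each add an InterpToMovement component at runtime to drive translation.
; When Rotate is set, Tick spins the actor locally at a fixed, delta-time-scaled rate, around roll if RotaX is set and yaw otherwise.
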(event EventBeginPlay
  (if (Variables|Default|Get¿UpnDown?)
    (AddComponent|AddInterptoMovementComponent))
  (if (Variables|Default|GetLeftAndRight?)
    (AddComponent|AddInterptoMovementComponent)))

(event EventTick
  (params (DeltaSeconds :type Float%20%28single-precision%29))
  (bind _returnvalue (* 200 DeltaSeconds))
  (if (Variables|Default|GetRotate?)
    (if (Variables|Default|GetRota%20X?)
      (Transformation|AddActorLocalRotation (Math|Rotator|MakeRotator _returnvalue 0.0 0.0) false false)
      (else
        (Transformation|AddActorLocalRotation (Math|Rotator|MakeRotator 0.0 0.0 _returnvalue) false false)))))

(fn ConstructionScript)