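; A player-operated elevator platform that moves up and down with the Elevator Up and Elevator Down input actions.
; A box overlap enables input while the FirstPersonCharacter stands inside and disables it on exit.
; The ArribaAbajo timeline lerps the platform between start and end locations, with an in-motion flag blocking new presses until it finishes.
; A ForzarBajada event reverses the timeline regardless of that flag, forcing a descent.
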(event OnComponentBeginOverlap(Box)
  (params (OverlappedComponent :type Primitive%20Component%20Object%20Reference) (OtherActor :type Actor%20Object%20Reference) (OtherComp :type Primitive%20Component%20Object%20Reference) (OtherBodyIndex :type Integer) (bFromSweep :type Boolean) (SweepResult :type Hit%20Result%20Structure%20%28by%20ref%29))
  ;[1 1 1] Control de Input
  (Utilities|Casting|CastToFirstPersonCharacter OtherActor)
  (Input|EnableInput (Game|GetPlayerController 0)))

(event OnComponentEndOverlap(Box)
  (params (OverlappedComponent :type Primitive%20Component%20Object%20Reference) (OtherActor :type Actor%20Object%20Reference) (OtherComp :type Primitive%20Component%20Object%20Reference) (OtherBodyIndex :type Integer))
  ;[1 1 1] Control de Input
  (Utilities|Casting|CastToFirstPersonCharacter OtherActor)
  (Input|DisableInput (Game|GetPlayerController 0)))

(event Custom|Forzar%20Bajada
  ;[1 1 1] Mov Ascensor
  (bind _alpha (Timeline|Arriba/Abajo Reverse)
    (:Update
      (Variables|Default|SetAscensorEnMovimiento true)
      (Transformation|SetRelativeLocation (Variables|Default|GetPlataformaAscensor) (Math|Vector|Lerp(Vector) (Variables|Default|GetInicioAscensor) (Variables|Default|GetFinAscensor) _alpha) false false))
    (:Finished
      (Variables|Default|SetAscensorEnMovimiento false))))

(event Input|ActionEvents|InputActionElevatorUp
  (params (Key :type Key%20Structure :default "None"))
  ;[1 1 1] Mov Ascensor
  (:Pressed
    (if (not (Variables|Default|GetAscensorEnMovimiento))
      (bind _alpha (Timeline|Arriba/Abajo Play)
        (:Update
          (Variables|Default|SetAscensorEnMovimiento true)
          (Transformation|SetRelativeLocation (Variables|Default|GetPlataformaAscensor) (Math|Vector|Lerp(Vector) (Variables|Default|GetInicioAscensor) (Variables|Default|GetFinAscensor) _alpha) false false))
        (:Finished
          (Variables|Default|SetAscensorEnMovimiento false))))))

(event Input|ActionEvents|InputActionElevatorDown
  (params (Key :type Key%20Structure :default "None"))
  ;[1 1 1] Mov Ascensor
  (:Pressed
    (if (not (Variables|Default|GetAscensorEnMovimiento))
      (bind _alpha (Timeline|Arriba/Abajo Reverse)
        (:Update
          (Variables|Default|SetAscensorEnMovimiento true)
          (Transformation|SetRelativeLocation (Variables|Default|GetPlataformaAscensor) (Math|Vector|Lerp(Vector) (Variables|Default|GetInicioAscensor) (Variables|Default|GetFinAscensor) _alpha) false false))
        (:Finished
          (Variables|Default|SetAscensorEnMovimiento false))))))

(fn ConstructionScript)