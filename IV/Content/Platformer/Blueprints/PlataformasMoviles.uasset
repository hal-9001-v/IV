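; PlataformasMoviles is a moving platform actor for a platformer, with movement selected by the UpnDown, LeftAndRight and Rotate flags.
; On BeginPlay, each enabled translation flag adds its own InterpToMovement component at runtime, with no path configured in the graph.
; When Rotate is set, Tick spins the actor around its local roll axis at a fixed, frame-rate-independent speed.
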(event EventBeginPlay
  (if (Variables|Default|Get¿UpnDown?)
    (AddComponent|AddInterptoMovementComponent))
  (if (Variables|Default|GetLeftAndRight?)
    (AddComponent|AddInterptoMovementComponent)))

(event Collision|EventActorBeginOverlap
  (params (OtherActor :type Actor%20Object%20Reference)))

(event EventTick
  (params (DeltaSeconds :type Float%20%28single-precision%29))
  (if (Variables|Default|GetRotate?)
    (Transformation|AddActorLocalRotation (Math|Rotator|MakeRotator (* 200 DeltaSeconds) 0.0 0.0) false false)))

(fn ConstructionScript)