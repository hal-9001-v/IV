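; Button actor that lets the player force an elevator down while standing in its trigger in the platformer.
; Overlapping ColisionBoton enables player input and ending the overlap disables it, for any actor; only FirstPersonCharacter also toggles the prompt text's visibility.
; The Elevator Down action calls ForzarBajada through three separate handlers, one each for the automatic, QE and final elevator references.
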(event OnComponentBeginOverlap(ColisionBoton)
  (params (OverlappedComponent :type Primitive%20Component%20Object%20Reference) (OtherActor :type Actor%20Object%20Reference) (OtherComp :type Primitive%20Component%20Object%20Reference) (OtherBodyIndex :type Integer) (bFromSweep :type Boolean) (SweepResult :type Hit%20Result%20Structure%20%28by%20ref%29))
  ;[0.03423 1 0.04394] Entrada en colisión y activar inputs
  (Input|EnableInput (Game|GetPlayerController 0))
  ;[0.4135 0.3222 0.04131] Aparicion y desaparicion de texto
  (Utilities|Casting|CastToFirstPersonCharacter OtherActor)
  (Rendering|ToggleVisibility (Variables|Default|GetTextRender) false))

(event OnComponentEndOverlap(ColisionBoton)
  (params (OverlappedComponent :type Primitive%20Component%20Object%20Reference) (OtherActor :type Actor%20Object%20Reference) (OtherComp :type Primitive%20Component%20Object%20Reference) (OtherBodyIndex :type Integer))
  ;[0.03423 1 0.04394] Entrada en colisión y activar inputs
  (Input|DisableInput (Game|GetPlayerController 0))
  ;[0.4135 0.3222 0.04131] Aparicion y desaparicion de texto
  (Utilities|Casting|CastToFirstPersonCharacter OtherActor)
  (Rendering|ToggleVisibility (Variables|Default|GetTextRender) false))

(event Input|ActionEvents|InputActionElevatorDown
  (params (Key :type Key%20Structure :default "None"))
  ;[0 0.09685 1] Bajada Elevador Automático
  (:Pressed
    (Default|ForzarBajada (Variables|Default|GetElevatorAutomático))))

(event Input|ActionEvents|InputActionElevatorDown
  (params (Key :type Key%20Structure :default "None"))
  ;[1 0 0] Bajada Elevador Final
  (:Pressed
    (Default|ForzarBajada (Variables|Default|GetElevatorFinal))))

(event Input|ActionEvents|InputActionElevatorDown
  (params (Key :type Key%20Structure :default "None"))
  ;[1 0 0.7789] Bajada Elevador QE
  (:Pressed
    (Default|ForzarBajada (Variables|Default|GetElevadorQE))))

(fn ConstructionScript)