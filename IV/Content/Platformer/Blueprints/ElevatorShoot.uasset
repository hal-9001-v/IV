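; Shootable elevator platform for the platformer that moves when its AciertoDiana (target hit) event is called.
; After a zero-length delay, the ArribaAbajo timeline drives a lerp of the platform's relative location between InicioAscensor and FinAscensor.
; The AscensorEnMovimiento flag, set during timeline updates and cleared on finish, ignores further hits while the platform moves.
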(event Custom|AciertoDiana
  ;[1 1 1] Mov Ascensor
  (if (not (Variables|Default|GetAscensorEnMovimiento))
    (Utilities|FlowControl|Delay 0.0)
    (bind _alpha (Timeline|Arriba/Abajo PlayFromStart)
      (:Update
        (Variables|Default|SetAscensorEnMovimiento true)
        (Transformation|SetRelativeLocation (Variables|Default|GetPlataformaAscensor) (Math|Vector|Lerp(Vector) (Variables|Default|GetInicioAscensor) (Variables|Default|GetFinAscensor) _alpha) false false))
      (:Finished
        (Variables|Default|SetAscensorEnMovimiento false)))))

(fn ConstructionScript)