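; BringThreeKeys is a message actor in a platformer that shows a request text until the player has collected three keys.
; Its Box trigger toggles the visibility of BringMeText whenever a FirstPersonCharacter begins or ends overlap.
; On Tick it polls the player character's KeysCollected and destroys itself once the count exceeds two.
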(event OnComponentBeginOverlap(Box)
  (params (OverlappedComponent :type Primitive%20Component%20Object%20Reference) (OtherActor :type Actor%20Object%20Reference) (OtherComp :type Primitive%20Component%20Object%20Reference) (OtherBodyIndex :type Integer) (bFromSweep :type Boolean) (SweepResult :type Hit%20Result%20Structure%20%28by%20ref%29))
  ;[0.4466 0.7852 1] Message Appears When Pkayer Near
  (Utilities|Casting|CastToFirstPersonCharacter OtherActor)
  (Rendering|ToggleVisibility (Variables|Default|GetBringMeText) false))

(event OnComponentEndOverlap(Box)
  (params (OverlappedComponent :type Primitive%20Component%20Object%20Reference) (OtherActor :type Actor%20Object%20Reference) (OtherComp :type Primitive%20Component%20Object%20Reference) (OtherBodyIndex :type Integer))
  ;[0.4466 0.7852 1] Message Appears When Pkayer Near
  (Utilities|Casting|CastToFirstPersonCharacter OtherActor)
  (Rendering|ToggleVisibility (Variables|Default|GetBringMeText) false))

(event EventTick
  (params (DeltaSeconds :type Float%20%28single-precision%29))
  ;[0.9974 0.162 1] Message Destroys When 3 Keys are collected
  (bind _asfirst_person_character (Utilities|Casting|CastToFirstPersonCharacter (Game|GetPlayerCharacter 0)))
  (if (> (Variables|/Game/FirstPersonBP/Blueprints/FirstPersonCharacter.FirstPersonCharacter_C|GetKeysCollected _asfirst_person_character) 2)
    (Actor|DestroyActor)))

(fn ConstructionScript)