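; Collectible key pickup for the Platformer content that spins in place until the player touches it.
; Tick adds a fixed local rotation each frame, without delta-time scaling.
; Collision overlap calls DestroyItem, which casts the actor to FirstPersonCharacter, increments its KeysCollected, plays the 1up sound and destroys the pickup.
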(event OnComponentBeginOverlap(collision)
  (params (OverlappedComponent :type Primitive%20Component%20Object%20Reference) (OtherActor :type Actor%20Object%20Reference) (OtherComp :type Primitive%20Component%20Object%20Reference) (OtherBodyIndex :type Integer) (bFromSweep :type Boolean) (SweepResult :type Hit%20Result%20Structure%20%28by%20ref%29))
  (CallFunction|DestroyItem OtherActor))

(event EventTick
  (params (DeltaSeconds :type Float%20%28single-precision%29))
  (Transformation|AddActorLocalRotation "0,5.000000, 0" false false))

(fn ConstructionScript)

(fn DestroyItem
  (params (Actor_Destroy :type Actor%20Object%20Reference))
  (bind _asfirst_person_character (Utilities|Casting|CastToFirstPersonCharacter Actor_Destroy))
  (Variables|/Game/FirstPersonBP/Blueprints/FirstPersonCharacter.FirstPersonCharacter_C|SetKeysCollected _asfirst_person_character (+ (Variables|/Game/FirstPersonBP/Blueprints/FirstPersonCharacter.FirstPersonCharacter_C|GetKeysCollected _asfirst_person_character) 1))
  (Audio|PlaySoundatLocation "/Game/SFX/1up.1up" (Transformation|GetActorLocation) "0, 0, 0" 1234312.0 1.0 0.0 0 0 0)
  (Actor|DestroyActor)
  (return false))