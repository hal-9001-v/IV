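; Automatic elevator for the first-person character, driven by a trigger box.
; Entering enables input and, after a delay, plays the ArribaAbajo timeline, lerping the platform between start and end locations.
; Leaving disables input and reverses the timeline after a shorter delay.
; A BotonBajarAscensorMariano with Id 1, found on BeginPlay, also reverses it through a dispatcher, which is bound every Tick.
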(event OnComponentBeginOverlap(Box)
  (params (OverlappedComponent :type Primitive%20Component%20Object%20Reference) (OtherActor :type Actor%20Object%20Reference) (OtherComp :type Primitive%20Component%20Object%20Reference) (OtherBodyIndex :type Integer) (bFromSweep :type Boolean) (SweepResult :type Hit%20Result%20Structure%20%28by%20ref%29))
  ;[0 0.8386 1] Control de Input
  (Utilities|Casting|CastToFirstPersonCharacter OtherActor)
  (Input|EnableInput (Game|GetPlayerController 0))
  ;[1 0.9936 0] Movimiento Ascensor
  (Utilities|FlowControl|Delay 1.5)
  (bind _alpha (Timeline|Arriba/Abajo Play)
    (:Update
      (Transformation|SetRelativeLocation (Variables|Default|GetPlataformaAscensor) (Math|Vector|Lerp(Vector) (Variables|Default|GetInicioAscensor) (Variables|Default|GetFinAscensor) _alpha) false false))))

(event OnComponentEndOverlap(Box)
  (params (OverlappedComponent :type Primitive%20Component%20Object%20Reference) (OtherActor :type Actor%20Object%20Reference) (OtherComp :type Primitive%20Component%20Object%20Reference) (OtherBodyIndex :type Integer))
  ;[0 0.8386 1] Control de Input
  (Utilities|Casting|CastToFirstPersonCharacter OtherActor)
  (Input|DisableInput (Game|GetPlayerController 0))
  ;[1 0.9936 0] Movimiento Ascensor
  (Utilities|FlowControl|Delay 0.5)
  (bind _alpha (Timeline|Arriba/Abajo Reverse)
    (:Update
      (Transformation|SetRelativeLocation (Variables|Default|GetPlataformaAscensor) (Math|Vector|Lerp(Vector) (Variables|Default|GetInicioAscensor) (Variables|Default|GetFinAscensor) _alpha) false false))))

(event Custom|BotonBajadaDispatcher_Event_1
  ;[1 0.1432 0.2973] BajadaForzosaBotón EMISION POR EVENTO
  ;[1 0.9936 0] Movimiento Ascensor
  (bind _alpha (Timeline|Arriba/Abajo Reverse)
    (:Update
      (Transformation|SetRelativeLocation (Variables|Default|GetPlataformaAscensor) (Math|Vector|Lerp(Vector) (Variables|Default|GetInicioAscensor) (Variables|Default|GetFinAscensor) _alpha) false false))))

(event EventTick
  (params (DeltaSeconds :type Float%20%28single-precision%29))
  ;[1 0.1432 0.2973] BajadaForzosaBotón EMISION POR EVENTO
  (EventDispatchers|AssignBotonBajadaDispatcher (Variables|Default|GetRefBoton) (delegate Custom|BotonBajadaDispatcher_Event_1)))

(event EventBeginPlay
  ;[1 0.1432 0.2973] BajadaForzosaBotón EMISION POR EVENTO
  (bind _outactors (Actor|GetAllActorsOfClass "/Game/Platformer/Blueprints/BotonBajarAscensorMariano.BotonBajarAscensorMariano_C"))
  (for _array_element _outactors
    (if (== (Variables|/Game/Platformer/Blueprints/BotonBajarAscensorMariano.BotonBajarAscensorMariano_C|GetId _array_element) 1)
      (Variables|Default|SetRefBoton _array_element))))

(fn ConstructionScript)